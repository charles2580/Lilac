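; Boss character that fights the player under an AI controller, passing the player and a one-time low-health flag to its Blackboard.
; Sword attack events start and stop a fast looping timer that line-traces between weapon sockets, dealing damage with a DoOnce cooldown and debug output.
; Incoming damage lowers HP and updates the boss health bar, which a sphere overlap creates and removes as the player enters and leaves.
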(event OnComponentBeginOverlap(Sphere)
  (params (OverlappedComponent :type Primitive%20Component%20Object%20Reference) (OtherActor :type Actor%20Object%20Reference) (OtherComp :type Primitive%20Component%20Object%20Reference) (OtherBodyIndex :type Integer) (bFromSweep :type Boolean) (SweepResult :type Hit%20Result%20Structure%20%28by%20ref%29))
  (bind _asbp_player (Utilities|Casting|CastToBP_Player OtherActor))
  (if (== _asbp_player (Game|GetPlayerCharacter 0))
    (bind _returnvalue (UserInterface|CreateWidget "/Game/Characters/Boss/WB_BossHealthBar.WB_BossHealthBar_C"))
    (bind _output_get (Variables|Default|SetBossHPBar _returnvalue))
    (Default|SetHPBar _output_get (Variables|Default|GetHP) (Variables|Default|GetMaxHP))
    (UserInterface|Viewport|AddtoViewport _output_get 0)))

(event OnComponentEndOverlap(Sphere)
  (params (OverlappedComponent :type Primitive%20Component%20Object%20Reference) (OtherActor :type Actor%20Object%20Reference) (OtherComp :type Primitive%20Component%20Object%20Reference) (OtherBodyIndex :type Integer))
  (Utilities|Casting|CastToBP_Player OtherActor)
  (Widget|RemovefromParent (Variables|Default|GetBossHPBar)))

(event Custom|TriggerSwordAttack
  (bind _returnvalue (Utilities|Time|SetTimerbyEvent (delegate Custom|SwordLineTrace) 0.001 true))
  (Variables|Default|SetSwordEvent _returnvalue))

(event Custom|SwordLineTrace
  (bind _mesh (Variables|Character|GetMesh))
  (bind (_outhit _returnvalue) (Collision|LineTraceByChannel (Transformation|GetSocketLocation _mesh "slashstart") (Transformation|GetSocketLocation _mesh "slasheffect") "TraceTypeQuery2" false 0 "ForDuration" true "(R=1.000000,G=0.000000,B=0.000000,A=1.000000)" "(R=0.000000,G=1.000000,B=0.000000,A=1.000000)" 2.0))
  (if _returnvalue
    (Utilities|FlowControl|DoOnce false :!label _label
      (:Completed
        (Game|Damage|ApplyDamage (.HitActor (Collision|BreakHitResult _outhit)) 2.0 0 self)
        (Development|PrintString "Attack" true true "(R=0.401775,G=1.000000,B=0.000000,A=1.000000)")
        (Utilities|FlowControl|Delay 1.0)
        (goto _label Reset)))))

(event Custom|StopTriggerSwordAttack
  (Utilities|Time|ClearandInvalidateTimerbyHandle (Variables|Default|GetSwordEvent)))

(event Custom|LowHealth)

(event EventBeginPlay
  (Transformation|AttachComponentToComponent (Variables|Default|GetSK_Blunt_MeatTenderizer) (Variables|Character|GetMesh) "Weaponmidle" "KeepRelative" "KeepRelative" "KeepRelative" true)
  (AI|Components|Blackboard|SetValueasObject (AI|GetBlackboard (AI|GetAIController self)) (Utilities|Name|MakeLiteralName "Player") (Game|GetPlayerCharacter 0)))

(event Collision|EventActorBeginOverlap
  (params (OtherActor :type Actor%20Object%20Reference)))

(event Game|Damage|EventAnyDamage
  (params (Damage :type Float%20%28single-precision%29) (DamageType :type Damage%20Type%20Object%20Reference) (InstigatedBy :type Controller%20Object%20Reference) (DamageCauser :type Actor%20Object%20Reference))
  (Utilities|FlowControl|Sequence
    (:then_0
      (bind _output_get (Variables|Default|SetHP (- (Variables|Default|GetHP) Damage)))
      (Default|SetHPBar (Variables|Default|GetBossHPBar) _output_get (Variables|Default|GetMaxHP)))
    (:then_1
      (if (< (Variables|Default|GetHP) 5e+01)
        (Utilities|FlowControl|DoOnce false
          (:Completed
            (AI|Components|Blackboard|SetValueasBool (AI|GetBlackboard (AI|GetAIController self)) (Utilities|Name|MakeLiteralName "LowHealth") true)))))))

(event EventTick
  (params (DeltaSeconds :type Float%20%28single-precision%29)))

(fn ConstructionScript)