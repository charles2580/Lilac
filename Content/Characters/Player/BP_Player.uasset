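; Player character Blueprint that handles sword hit detection for melee attacks.
; TriggerSword starts a fast looping timer that line-traces between the right blade's Start and End sockets on the Camera channel with debug drawing, until StopTriggerSword clears it.
; Every trace applies damage to the hit actor; the DoOnce and delay throttle only the debug "Attack" print.
; The combo montage playback logic is unconnected and never runs.
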(event Custom|TriggerSword
  (bind _returnvalue (Utilities|Time|SetTimerbyEvent (delegate Custom|SwordLineTrace) 0.001 true))
  (Variables|Default|SetTriggerSwordEvent _returnvalue))

(event Custom|SwordLineTrace
  (bind _grruzam_modeling_dualblade_r (Variables|Default|GetGrruzam_Modeling_DualBlade_R))
  (bind _outhit (Collision|LineTraceByChannel (Transformation|GetSocketLocation _grruzam_modeling_dualblade_r "Start") (Transformation|GetSocketLocation _grruzam_modeling_dualblade_r "End") "TraceTypeQuery2" false 0 "ForDuration" true "(R=1.000000,G=0.000000,B=0.000000,A=1.000000)" "(R=0.000000,G=1.000000,B=0.000000,A=1.000000)" 2.0))
  (Game|Damage|ApplyDamage (.HitActor (Collision|BreakHitResult _outhit)) 1.0 0 0)
  (Utilities|FlowControl|DoOnce false :!label _label
    (:Completed
      (Development|PrintString "Attack" true true "(R=0.401775,G=1.000000,B=0.000000,A=1.000000)")
      (Utilities|FlowControl|Delay 0.2)
      (goto _label Reset))))

(event Custom|StopTriggerSword
  (Utilities|Time|ClearandInvalidateTimerbyHandle (Variables|Default|GetTriggerSwordEvent)))

(event Collision|EventActorBeginOverlap
  (params (OtherActor :type Actor%20Object%20Reference)))

(event EventTick
  (params (DeltaSeconds :type Float%20%28single-precision%29)))

(event Input|MouseEvents|LeftMouseButton
  (params (Key :type Key%20Structure :default "None")))

(fn ConstructionScript)